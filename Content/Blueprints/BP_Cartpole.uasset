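; BP_Cartpole is a test-style actor Blueprint, named for a cartpole, that exchanges state and input through UpdateState and UseInput.
; It sends an array of three random floats to UpdateState on BeginPlay and again every Tick, in place of real simulation values.
; Each Tick first calls UseInput and prints the length of the result when it is non-empty, without otherwise acting on it.
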(event EventBeginPlay
  (bind _returnvalue (Math|Random|RandomFloat))
  (Class|Cartpole|UpdateState (Utilities|Array|MakeArray _returnvalue _returnvalue _returnvalue)))

(event Collision|EventActorBeginOverlap
  (params (OtherActor :type Actor%20Object%20Reference)))

(event EventTick
  (params (DeltaSeconds :type Float%20%28single-precision%29))
  (bind _returnvalue (Math|Random|RandomFloat))
  (bind _a_out (Class|Cartpole|UseInput))
  (Utilities|FlowControl|Sequence
    (:then_0
      (if (!= (Utilities|Array|Length _a_out) 0)
        (Development|PrintString (Utilities|String|ToString(Integer) (Utilities|Array|Length _a_out)))))
    (:then_1
      (Class|Cartpole|UpdateState (Utilities|Array|MakeArray _returnvalue _returnvalue _returnvalue)))))

(fn ConstructionScript)