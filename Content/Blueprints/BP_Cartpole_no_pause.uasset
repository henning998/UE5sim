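; Cart-pole environment for a learning agent, built on physics bodies, that steps every Tick without pausing the simulation.
; A two-value input picks a left or right impulse on the cart, then reward accrues until position, tilt or step limits end the episode.
; Cart position, pole pitch and cached velocities form the state; only Pause refreshes those velocities via SaveVelocity.
; ResetEnv recenters the cart's X, randomizes pole tilt and clears counters.
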(event EventBeginPlay
  (CallFunction|SetState))

(event Collision|EventActorBeginOverlap
  (params (OtherActor :type Actor%20Object%20Reference)))

(event EventTick
  (params (DeltaSeconds :type Float%20%28single-precision%29))
  (bind _done (Class|Cartpole|GetDone))
  (if (not _done)
    (bind _a_out (Class|Cartpole|UseInput))
    (if (== (Utilities|Array|Length _a_out) 2)
      (bind _done_2 (Class|Cartpole|GetDone))
      (if (not _done_2)
        (Math|Float|CompareFloat (Utilities|Array|Get(acopy) _a_out) (Utilities|Array|Get(acopy) _a_out 1)
          (:>
            (Physics|AddImpulse (Variables|Default|GetCube) "100.000000,0.000000, 0" "None" true))
          (:==
            (Physics|AddImpulse (Variables|Default|GetCube) "0, 0, 0" "None" true))
          (:<
            (Physics|AddImpulse (Variables|Default|GetCube) "-100.000000,0.000000, 0" "None" true)))
        (CallFunction|CalculateRewardandDone)
        (CallFunction|SetState)))))

(event EventResetEnv
  (bind _y (Class|Cartpole|GetYLocation))
  (Transformation|SetWorldLocation (Variables|Default|GetCube) (Math|Vector|MakeVector 0.0 _y 5.0) false true)
  (Variables|Default|SetCubeVelocity "0, 0, 0")
  (Variables|Default|SetPoleangelvelocity "0, 0, 0")
  (Variables|Default|SetReward 0.0)
  (Variables|Default|SetSteps 0)
  (bind _rot_out (Class|Cartpole|SetRandomStartRotation))
  (Transformation|SetRelativeRotation (Variables|Default|GetCylinder) _rot_out false false)
  (Class|Cartpole|SetDone false)
  (Class|Cartpole|UpdateState (Utilities|Array|MakeArray (.x (Transformation|GetWorldLocation (Variables|Default|GetCube))) (.x (Variables|Default|GetCubeVelocity)) (.pitch (Variables|/Script/Engine.SceneComponent|GetRelativeRotation (Variables|Default|GetCylinder))) (.y (Variables|Default|GetPoleangelvelocity))) true))

(event EventPause
  (CallFunction|SaveVelocity)
  (Variables|Default|SetAgentPause true)
  (Physics|SetSimulatePhysics (Variables|Default|GetSphere) false)
  (Physics|SetSimulatePhysics (Variables|Default|GetCylinder) false)
  (Physics|SetSimulatePhysics (Variables|Default|GetCube) false))

(event EventResume
  (CallFunction|SetVelocity)
  (Variables|Default|SetAgentPause false)
  (Physics|SetSimulatePhysics (Variables|Default|GetSphere) true)
  (Physics|SetSimulatePhysics (Variables|Default|GetCylinder) true)
  (Physics|SetSimulatePhysics (Variables|Default|GetCube) true))

(fn ConstructionScript
  (bind _rot_out (Class|Cartpole|SetRandomStartRotation))
  (Transformation|SetRelativeRotation (Variables|Default|GetSphere) _rot_out false false))

(fn Test
  (bind _a_out (Class|Cartpole|UseInput))
  (Utilities|FlowControl|Sequence
    (:then_0
      (if (== (Utilities|Array|Length _a_out) 2)
        (Development|PrintString (Utilities|String|ToString(Integer) (Utilities|Array|Length _a_out)))))))

(fn SaveVelocity
  (bind _cube (Variables|Default|GetCube))
  (bind _returnvalue (Physics|GetPhysicsLinearVelocity _cube "None"))
  (if (Physics|IsSimulatingPhysics _cube "None")
    (Variables|Default|SetCubeVelocity _returnvalue)
    (Variables|Default|SetPoleangelvelocity (Physics|GetPhysicsAngularVelocityinDegrees (Variables|Default|GetCylinder) "None"))))

(fn SetVelocity
  (Physics|SetPhysicsLinearVelocity (Variables|Default|GetCube) (Variables|Default|GetCubeVelocity) false "None")
  (Class|PrimitiveComponent|SetPhysicsAngularVelocityinDegrees (Variables|Default|GetCylinder) (Variables|Default|GetPoleangelvelocity) false "None"))

(fn CalculateRewardandDone
  (bind _cube (Variables|Default|GetCube))
  (bind _cylinder (Variables|Default|GetCylinder))
  (bind _returnvalue (Transformation|GetWorldLocation _cube))
  (bind _returnvalue_2 (Transformation|GetWorldRotation _cylinder))
  (if (and (<= (.x _returnvalue) 1.5e+03) (>= (.x _returnvalue) -1.5e+03))
    (if (and (<= (.pitch _returnvalue_2) 35.0) (>= (.pitch _returnvalue_2) -35.0))
      (if (<= (Variables|Default|GetSteps) 500)
        (bind _result (Math|Float|IncrementFloat (Variables|Default|GetReward))
          (:%20%20
            (Variables|Default|SetReward _result)
            (Class|Cartpole|SetDone false)
            (bind _result_2 (Math|Integer|IncrementInt (Variables|Default|GetSteps))
              (:%20%20
                (Variables|Default|SetSteps _result_2)))))
        (else
          (Class|Cartpole|SetDone true :!label _label)
          (Class|Cartpole|SetReward (Variables|Default|GetReward))))
      (else
        (goto _label)))
    (else
      (goto _label))))

(fn SetState
  (Class|Cartpole|UpdateState (Utilities|Array|MakeArray (.x (Transformation|GetWorldLocation (Variables|Default|GetCube))) (.x (Variables|Default|GetCubeVelocity)) (.pitch (Variables|/Script/Engine.SceneComponent|GetRelativeRotation (Variables|Default|GetCylinder))) (.y (Variables|Default|GetPoleangelvelocity))) false))